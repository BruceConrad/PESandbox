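; A configurable exhaust effect Blueprint that tints a mesh, particle effect and light with one shared color.
; The construction script creates a dynamic material from PE_My_Material on MyMesh, then pushes MainColor to that material, the MyExhaust particles and MyLight.
; It also sets the material's speed from MainSpeed and the particles' smoke from SmokeEmit.
; All setup happens at construction, with no active runtime logic in the event graph.
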(fn `UserConstructionScript`
  (bind _exhaust_material (`self.Exhaust_Material`))
  (bind _maincolor (`self.MainColor`))
  (bind _my_exhaust (`self.My_Exhaust`))
  (bind _returnvalue (`PrimitiveComponent.CreateDynamicMaterialInstance` (`self.My_Mesh`) 0 "/Game/PE_My_Material.PE_My_Material" "None"))
  (set `self.Exhaust_Material` _returnvalue)
  (`MaterialInstanceDynamic.SetVectorParameterValue` _exhaust_material "Color" _maincolor)
  (`FXSystemComponent.SetColorParameter` _my_exhaust "Color" _maincolor)
  (`LightComponent.SetLightColor` (`self.My_Light`) _maincolor true)
  (`MaterialInstanceDynamic.SetScalarParameterValue` _exhaust_material "MainSpeed" (`self.MainSpeed`))
  (`FXSystemComponent.SetFloatParameter` _my_exhaust "Smoke" (`self.SmokeEmit`)))